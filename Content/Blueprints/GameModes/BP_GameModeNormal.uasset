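; Game mode that runs endless waves of aliens, scaling the alien count by a difficulty multiplier each wave.
; Looping timers spawn aliens at random TargetPoints and a random number of health pickups at BP_HealthPickupSpawn points.
; Used pickup points are recorded and never cleared, so each is used only once.
; RegisterAlienDeath starts the next wave after a short delay once no living or pending aliens remain.
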(event `self.ReceiveBeginPlay`
  (`KismetSystemLibrary.Delay` 2.0)
  (`self.Start New Wave`))

(event `Spawn Wave`
  (`self.Spawn Alien`))

(event `Spawn Health`
  (`self.Spawn Health Pickups`))

(event `End Wave`
  (`KismetSystemLibrary.Delay` 2.0)
  (`self.Start New Wave`))

(fn `Get Random Alien Spawn Point`
  (returns (`Spawn Point` :type "TargetPoint Object Reference"))
  (bind _outactors (`GameplayStatics.GetAllActorsOfClass` "/Script/Engine.TargetPoint"))
  (return (`|GetArrayItem` _outactors (`KismetMathLibrary.RandomIntegerInRange` 0 (`KismetArrayLibrary.Array_LastIndex` _outactors)))))

(fn `Get Random Health Pickup Spawn Point`
  (returns (`Spawn Point` :type "/Game/Blueprints/Pickups/BP_HealthPickupSpawn Object Reference"))
  (bind _outactors (`GameplayStatics.GetAllActorsOfClass` "/Game/Blueprints/Pickups/BP_HealthPickupSpawn.BP_HealthPickupSpawn_C"))
  (return (`|GetArrayItem` _outactors (`KismetMathLibrary.RandomIntegerInRange` 0 (- (`KismetArrayLibrary.Array_Length` _outactors) 1)))))

(fn `Increase Wave Difficulty`
  (bind _output_get (set `self.Wave Difficulty` (`KismetMathLibrary.Round` (* (`self.Wave Difficulty`) (`self.Difficulty Multiplier`)))))
  (set `self.Alien Spawns Remaining` _output_get)
  (set `self.Health Spawns Remaining` (`KismetMathLibrary.RandomIntegerInRange` 0 (/ (`self.Wave Difficulty`) 4)))
  (`KismetSystemLibrary.PrintString` (`KismetStringLibrary.Conv_IntToString` (`self.Health Spawns Remaining`))))

(fn `Is Spawn Location Used?`
  (params (`Spawn Point` :type "/Game/Blueprints/Pickups/BP_HealthPickupSpawn Object Reference (by ref)"))
  (returns (ValidLocation :type Boolean))
  (return (== (`KismetArrayLibrary.Array_Find` (`self.Previous Spawn Locations`) `Spawn Point`) -1)))

(fn `Is Wave Complete`
  (returns (ReturnValue :type Boolean))
  (return (and (== (`KismetArrayLibrary.Array_Length` (`self.Aliens`)) 0) (== (`self.Alien Spawns Remaining`) 0))))

(fn `Register Alien Death`
  (params (Alien :type "/Game/Blueprints/AI/BP_Alien Object Reference (by ref)"))
  (`KismetArrayLibrary.Array_RemoveItem` (`self.Aliens`) Alien)
  (if (`self.Is Wave Complete`)
    (`self.End Wave`)))

(fn `Spawn Alien`
  (bind _spawn_point (`self.Get Random Alien Spawn Point`))
  (`/Engine/EditorBlueprintResources/StandardMacros.IsValid` _spawn_point
    (:`Is Valid`
      (bind _returnvalue (`|SpawnActorFromClass` "/Game/Blueprints/AI/BP_Alien.BP_Alien_C" (`self.GetTransform` _spawn_point) "Undefined" "OverrideRootScale" null null))
      (`/Engine/EditorBlueprintResources/StandardMacros.IsValid` _returnvalue
        (:`Is Valid`
          (`KismetArrayLibrary.Array_Add` (`self.Aliens`) _returnvalue)
          (bind _result (`/Engine/EditorBlueprintResources/StandardMacros.DecrementInt` (`self.Alien Spawns Remaining`))
            (:`  `
              (if (== _result 0)
                (`KismetSystemLibrary.K2_ClearTimer` null "Spawn Wave")))))))))

(fn `Spawn Health Pickups`
  (bind _spawn_point (`self.Get Random Health Pickup Spawn Point`))
  (`/Engine/EditorBlueprintResources/StandardMacros.IsValid` _spawn_point
    (:`Is Valid`
      (if (`self.Is Spawn Location Used?` _spawn_point)
        (bind _returnvalue (`|SpawnActorFromClass` "/Game/Blueprints/Pickups/BP_HealthPickup.BP_HealthPickup_C" (`self.GetTransform` _spawn_point) "Undefined" "OverrideRootScale" null null))
        (`/Engine/EditorBlueprintResources/StandardMacros.IsValid` _returnvalue
          (:`Is Valid`
            (`/Engine/EditorBlueprintResources/StandardMacros.DecrementInt` (`self.Health Spawns Remaining`)
              (:`  `
                (`KismetArrayLibrary.Array_Add` (`self.Previous Spawn Locations`) _spawn_point)
                (if (== (`self.Health Spawns Remaining`) 0)
                  (`KismetSystemLibrary.K2_ClearTimer` null "Spawn Health"))))))))))

(fn `Start New Wave`
  (`/Engine/EditorBlueprintResources/StandardMacros.IncrementInt` (`self.Current Wave`)
    (:`  `
      (`self.Increase Wave Difficulty`)
      (`KismetSystemLibrary.K2_SetTimer` null "Spawn Wave" (`self.Spawn Frequency`) true)
      (`KismetSystemLibrary.K2_SetTimer` null "Spawn Health" (`self.Health Spawn Frequency`) true))))

(fn `UserConstructionScript`)