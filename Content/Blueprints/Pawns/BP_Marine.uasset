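; BP_Marine is the player pawn for a shooter against aliens, with world-axis movement, HUD, health and kill count.
; Tick aims control rotation from thumbstick or smoothed mouse velocity, following the last key's device.
; Firing loops a timed muzzle line trace that applies damage and spawns alien-specific or generic impacts.
; At zero health it handles death; one HandleDeath graph fades and reloads the level, another only fades and sets Dead false.
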(event `self.ReceiveBeginPlay`
  (bind _returnvalue (`|CreateWidget` "/Game/UI/W_PlayerHUD.W_PlayerHUD_C" null self))
  (`UserWidget.AddToViewport` _returnvalue 0))

(event `InputAxis|MoveForward`
  (params (AxisValue :type "Float (single-precision)"))
  (if (`self.Is Alive`)
    (`self.AddMovementInput` (1.0 0.0 0.0) AxisValue)))

(event `InputAxis|MoveRight`
  (params (AxisValue :type "Float (single-precision)"))
  (if (`self.Is Alive`)
    (`self.AddMovementInput` (0.0 1.0 0.0) AxisValue)))

(event `self.ReceiveTick`
  (params (DeltaSeconds :type "Float (single-precision)"))
  (`self.Update Player Aim`))

(event `Key|AnyKey`
  (params (Key :type "Key Structure"))
  (:`Pressed`
    (set `self.IsGamepadActive` (`KismetInputLibrary.Key_IsGamepadKey` Key))))

(event `InputAction|FireWeapon`
  (params (Key :type "Key Structure"))
  (:`Pressed`
    (`self.Start Firing Weapon`))
  (:`Released`
    (`self.Stop Firing Weapon`)))

(event `self.ReceiveAnyDamage`
  (params (Damage :type "Float (single-precision)") (DamageType :type "DamageType Object Reference") (InstigatedBy :type "Controller Object Reference") (DamageCauser :type "Actor Object Reference"))
  (bind _health (`self.Decrease Health` Damage))
  (if (== _health 0.0)
    (`self.HandleDeath`)))

(fn `Add Health`
  (params (HealthToAdd :type "Float (double-precision)"))
  (set `self.Health` (`KismetMathLibrary.FClamp` (+ HealthToAdd (`self.Health`)) 0.0 100.0)))

(fn `Decrease Health`
  (params (`Damage Amount` :type "Float (double-precision)"))
  (returns (Health :type "Float (double-precision)"))
  (bind _output_get (set `self.Health` (`KismetMathLibrary.FClamp` (- (`self.Health`) `Damage Amount`) 0.0 100.0)))
  (return _output_get))

(fn `Get Mouse Aim Direction`
  (returns (ReturnValue :type "Rotator Structure"))
  (bind (_returnvalue_x _returnvalue_y) (`KismetMathLibrary.BreakVector2D` (`self.Get Mouse Velocity`)))
  (return (`KismetMathLibrary.RInterpTo` (`Controller.GetControlRotation` (`GameplayStatics.GetPlayerController` 0)) (`KismetMathLibrary.MakeRotator` 0.0 0.0 (`KismetMathLibrary.DegAtan2` _returnvalue_x _returnvalue_y)) (`GameplayStatics.GetWorldDeltaSeconds`) (`self.Mouse Smoothing Strength`))))

(fn `Get Mouse Velocity`
  (returns (ReturnValue :type "Vector2D Structure"))
  (bind (_deltax _deltay) (`PlayerController.GetInputMouseDelta` (`GameplayStatics.GetPlayerController` 0)))
  (return (/ (`KismetMathLibrary.MakeVector2D` _deltax _deltay) (`GameplayStatics.GetWorldDeltaSeconds`))))

(fn `Get Thumbstick Aim Direction`
  (returns (NewRotator :type "Rotator Structure"))
  (return (`KismetMathLibrary.MakeRotator` 0.0 0.0 (`KismetMathLibrary.DegAtan2` (`self.GetInputAxisValue`) (`self.GetInputAxisValue`)))))

(fn `Get Weapon Trace End Location`
  (returns (ReturnValue :type "Vector Structure"))
  (return (+ (`self.Get Weapon Trace Start Location`) (* (`KismetMathLibrary.GetForwardVector` (`self.GetControlRotation`)) (`self.Weapon Range`)))))

(fn `Get Weapon Trace Start Location`
  (returns (ReturnValue :type "Vector Structure"))
  (return (`SceneComponent.GetSocketLocation` (`self.RifleMesh`) "MuzzleFlash")))

(fn `Handle Death`
  (set `self.Dead` false)
  (`self.Stop Firing Weapon`)
  (`PlayerCameraManager.StartCameraFade` :`self` (`GameplayStatics.GetPlayerCameraManager` 0) :`ToAlpha` 1.0 :`Duration` (`self.Fade Duration`)))

(fn `Increase Kills`
  (`/Engine/EditorBlueprintResources/StandardMacros.IncrementInt` (`self.KillCount`)))

(fn `Is Alive`
  (returns (ReturnValue :type Boolean))
  (return (not (`self.Dead`))))

(fn `Is Health Full`
  (returns (ReturnValue :type Boolean))
  (return (== (`self.Health`) 100.0)))

(fn `Is Mouse Above Deadzone`
  (returns (ReturnValue :type Boolean))
  (return (> (`KismetMathLibrary.VSize2D` (`self.Get Mouse Velocity`)) (`self.Mouse Deadzone`))))

(fn `Is Thumbstick Above Deadzone`
  (returns (ReturnValue :type Boolean))
  (return (> (`KismetMathLibrary.VSize2D` (`KismetMathLibrary.MakeVector2D` (`self.GetInputAxisValue`) (`self.GetInputAxisValue`))) (`self.Thumbstick Deadzone`))))

(fn `IsMoving`
  (returns (`Is Moving` :type Boolean))
  (return (> (`KismetMathLibrary.VSize` (`self.GetVelocity` self)) 0.0)))

(fn `Spawn Impact Hit - Alien`
  (params (HitLocation :type "Vector Structure"))
  (`GameplayStatics.SpawnEmitterAtLocation` "/Game/Effects/Weapons/Impacts/P_CreatureImpact.P_CreatureImpact" HitLocation))

(fn `Spawn Impact Hit - Other`
  (params (HitLocation :type "Vector Structure"))
  (`GameplayStatics.SpawnEmitterAtLocation` "/Game/Effects/Weapons/Impacts/P_AssaultRifle_IH.P_AssaultRifle_IH" HitLocation))

(fn `Start Firing Weapon`
  (if (`self.Is Alive`)
    (`ActorComponent.Activate` (`self.P_AssaultRifle_MF`) false)
    (bind _returnvalue (`GameplayStatics.SpawnSound2D` "/Game/Sounds/Weapon_AssaultRifle/Stereo/RifleFireLoop_Cue.RifleFireLoop_Cue" 1.0 1.0 0.0 null))
    (set `self.Weapon Fire Sound` _returnvalue)
    (`self.Weapon Trace`)
    (`KismetSystemLibrary.K2_SetTimer` null "Weapon Trace" (`self.Weapon Fire Rate`) true)))

(fn `Stop Firing Weapon`
  (bind _weapon_fire_sound (`self.Weapon Fire Sound`))
  (`ActorComponent.Deactivate` (`self.P_AssaultRifle_MF`))
  (`/Engine/EditorBlueprintResources/StandardMacros.IsValid` _weapon_fire_sound
    (:`Is Valid`
      (`AudioComponent.Stop` _weapon_fire_sound)
      (`KismetSystemLibrary.K2_ClearTimer` null "Weapon Trace")
      (if (`self.Is Alive`)
        (`GameplayStatics.SpawnSound2D` "/Game/Sounds/Weapon_AssaultRifle/Stereo/RifleFireEnd_Cue.RifleFireEnd_Cue" 1.0 1.0 0.0 null)))))

(fn `Update Mouse Aim`
  (if (`self.Is Mouse Above Deadzone`)
    (`Controller.SetControlRotation` (`GameplayStatics.GetPlayerController` 0) (`self.Get Mouse Aim Direction`))))

(fn `Update Player Aim`
  (if (`self.Is Alive`)
    (if (`self.IsGamepadActive`)
      (`self.Update Thumbstick Aim`)
      (else
        (`self.Update Mouse Aim`)))))

(fn `Update Thumbstick Aim`
  (if (`self.Is Thumbstick Above Deadzone`)
    (`Controller.SetControlRotation` (`GameplayStatics.GetPlayerController` 0) (`self.Get Thumbstick Aim Direction`))))

(fn `UserConstructionScript`)

(fn `Weapon Trace`
  (bind _outhit (`KismetSystemLibrary.LineTraceSingle` :`Start` (`self.Get Weapon Trace Start Location`) :`End` (`self.Get Weapon Trace End Location`) :`TraceChannel` "TraceTypeQuery1" :`DrawTime` 2.0))
  (bind (_bblockinghit _binitialoverlap _time _distance _location _impactpoint _normal _impactnormal _physmat _hitactor) (`GameplayStatics.BreakHitResult` _outhit))
  (if _bblockinghit
    (`GameplayStatics.ApplyDamage` _hitactor (`self.Damage Per Shot`))
    (cast `/Game/Blueprints/AI/BP_Alien` _hitactor
      (:`then`
        (`self.Spawn Impact Hit - Alien` _location)
        (`GameplayStatics.SpawnSoundAtLocation` "/Game/Sounds/FoleyFlesh/Mono/FoleyFlesh_Impact_Cue.FoleyFlesh_Impact_Cue" _location (struct) 1.0 1.0 0.0 null null))
      (:`CastFailed`
        (`self.Spawn Impact Hit - Other` _location)))))